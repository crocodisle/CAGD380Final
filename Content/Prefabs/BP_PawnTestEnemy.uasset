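; BP_PawnTestEnemy is a test enemy that homes in on the player character.
; It caches player character 0 on BeginPlay, then each Tick snaps its transform to face that target via LookAt with a fixed up vector.
; It then moves along local forward by MoveSpeed per frame, without sweep or delta-time scaling.
; An alternative yaw-turning step using TurnSpeed is left unconnected.
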(event `self.ReceiveBeginPlay`
  (set `self.Target` (`GameplayStatics.GetPlayerCharacter` 0)))

(event `self.ReceiveTick`
  (params (DeltaSeconds :type "Float (single-precision)"))
  (`self.K2_SetActorTransform` (`KismetAnimationLibrary.K2_LookAt` (`self.GetTransform`) (`self.K2_GetActorLocation` (`self.Target`)) (1.0 0.0 0.0) true (0.0 0.0 1.0)))
  (`self.K2_AddActorLocalOffset` (* (1.0 0.0 0.0) (`self.MoveSpeed`))))

(fn `UserConstructionScript`)