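; BP_ProjectileBase is a projectile that flies forward each tick with a swept move and damages what it overlaps, ignoring Player-tagged actors.
; Targets with a BP_StatComponent lose health by the instigating third-person character's MagicPower or ShotDamage, chosen by the Magical flag, and are destroyed at zero.
; Targets without one are destroyed if tagged Generator or Pickup; other non-player overlaps generally just destroy the projectile.
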(event `self.ReceiveTick`
  (params (DeltaSeconds :type "Float (single-precision)"))
  (`self.K2_AddActorLocalOffset` (* (`self.Speed`) (`KismetMathLibrary.Vector_Forward`)) true))

(event `self.Sphere.OnComponentBeginOverlap`
  (params (OverlappedComponent :type "PrimitiveComponent Object Reference") (OtherActor :type "Actor Object Reference") (OtherComp :type "PrimitiveComponent Object Reference") (OtherBodyIndex :type Integer) (bFromSweep :type Boolean) (SweepResult :type "HitResult Structure (by ref)"))
  (bind _returnvalue (`self.GetComponentByClass` OtherActor "/Game/Prefabs/BP_StatComponent.BP_StatComponent_C"))
  (bind _health (`/Game/Prefabs/BP_StatComponent.Health` _returnvalue))
  (if (not (`KismetArrayLibrary.Array_Contains` (`Actor.Tags` OtherActor) "Player"))
    (if (`KismetSystemLibrary.IsValid` _returnvalue)
      (bind _asbp_third_person_character (cast `/Game/ThirdPerson/Blueprints/BP_ThirdPersonCharacter` (`self.GetInstigator`)))
      (if (`self.Magical`)
        (bind _bp_statcomponent (`/Game/ThirdPerson/Blueprints/BP_ThirdPersonCharacter.BP_StatComponent` _asbp_third_person_character))
        (bind _output_get (set `/Game/Prefabs/BP_StatComponent.Health` (`KismetMathLibrary.FTrunc` (- _health (`/Game/Prefabs/BP_StatComponent.Magic Power` _bp_statcomponent))) _returnvalue))
        (`KismetSystemLibrary.PrintString` (`KismetStringLibrary.Conv_IntToString` _output_get))
        (if (<= _output_get 0)
          (`self.K2_DestroyActor` OtherActor))
        (else
          (bind _output_get_2 (set `/Game/Prefabs/BP_StatComponent.Health` (`KismetMathLibrary.FTrunc` (- _health (`/Game/Prefabs/BP_StatComponent.Shot Damage` _bp_statcomponent))) _returnvalue))
          (`KismetSystemLibrary.PrintString` (`KismetStringLibrary.Conv_IntToString` _output_get_2))
          (if (<= _output_get_2 0)
            (`self.K2_DestroyActor` OtherActor :!label _label)
            (if (`self.ActorHasTag` OtherActor "Pickup") :!label _label_2
              (goto _label)
              (else
                _)))))
      (elif (`self.ActorHasTag` OtherActor "Generator")
        (goto _label)
        (else
          (goto _label_2))))
    (`self.K2_DestroyActor`)))

(fn `UserConstructionScript`)